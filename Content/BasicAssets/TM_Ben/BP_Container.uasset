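; BP_Container is a box that tries to capture BP_Cat actors overlapping it.
; Acceptance requires the cat to be above the entrance point and pass a unit-versus-capacity check, which tests cat units >= remaining space.
; Accepted cats join HeldCats, while rejected ones get a randomized force at the entrance.
; Enable and disable are print-string stubs, and removal, which teleports cats to an exit point, is never triggered.
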(event EventBeginPlay)

(event Collision|EventActorBeginOverlap
  (params (OtherActor :type Actor%20Object%20Reference))
  (bind _asbp_cat (Utilities|Casting|CastToBP_Cat OtherActor))
  (bind _added_succesfully (CallFunction|TryAddCattoBox _asbp_cat))
  (if _added_succesfully
    (CallFunction|AcceptCat _asbp_cat)
    (else
      (CallFunction|RejectCat _asbp_cat))))

(event EventTick
  (params (DeltaSeconds :type Float%20%28single-precision%29)))

(fn ConstructionScript)

(fn TryAddCattoBox
  (params (Query%20Cat :type BP%20Cat%20Object%20Reference))
  (Utilities|FlowControl|Sequence
    (:then_0
      (bind _has_room (CallFunction|DoesBoxHaveRoomforCat? Query%20Cat)))
    (:then_1
      (bind _above_hole (CallFunction|IsCatAboveBoxHole? Query%20Cat)))
    (:then_2
      (return (and _above_hole _has_room)))))

(fn RemoveCatfromBox
  (params (Cat :type BP%20Cat%20Object%20Reference))
  (Utilities|Set|Remove (Variables|Default|GetHeld%20Cats) Cat)
  (CallFunction|EnableCat Cat)
  (Transformation|SetActorLocation Cat (Transformation|GetWorldLocation (Variables|Default|GetBox%20Exit%20%28For%20Cat%20Locations%29)) false true))

(fn GetRemainingCatAmounts
  (return (- (Variables|Default|GetMax%20Cat%20Amount) (Variables|Default|GetCurrent%20Cat%20Amount))))

(fn EnableCat
  (params (Target%20Cat :type BP%20Cat%20Object%20Reference))
  (Development|PrintString "Enable physics onthe cat and show its mesh!" true true "(R=0.000000,G=0.660000,B=1.000000,A=1.000000)" 25.0))

(fn DisableCat
  (params (Target%20Cat :type BP%20Cat%20Object%20Reference))
  (Development|PrintString "Disable physics on the cat and hide its mesh!" true true "(R=0.000000,G=0.660000,B=1.000000,A=1.000000)" 25.0))

(fn CanAddCattoBox
  (params (Query :type BP%20Cat%20Object%20Reference)))

(fn DoesBoxHaveRoomforCat?
  (params (Query :type BP%20Cat%20Object%20Reference))
  (bind _amount (CallFunction|GetRemainingCatAmounts))
  (bind _units (Default|GetCatUnits Query))
  (return (>= _units _amount)))

(fn IsCatAboveBoxHole?
  (params (Query :type BP%20Cat%20Object%20Reference))
  (return (> (.z (Transformation|GetActorLocation Query)) (.z (Transformation|GetWorldLocation (Variables|Default|GetBox%20Entrance%20%28For%20Hole%20Detection%29))))))

(fn RejectCat
  (params (Cat :type BP%20Cat%20Object%20Reference))
  (bind _reject_lateral_force (Variables|Default|GetReject%20Lateral%20Force))
  (Class|PrimitiveComponent|AddForceatLocation (Variables|/Game/BasicAssets/Cat/BP_Cat.BP_Cat_C|GetCat Cat) (Math|Vector|MakeVector (* (Math|Random|RandomFloat) _reject_lateral_force) (* _reject_lateral_force (Math|Random|RandomFloat)) (* (Variables|Default|GetReject%20Up%20Force) (Math|Random|RandomFloat))) (Transformation|GetWorldLocation (Variables|Default|GetBox%20Entrance%20%28For%20Hole%20Detection%29)) "None"))

(fn AcceptCat
  (params (Cat :type BP%20Cat%20Object%20Reference))
  (Utilities|Set|Add (Variables|Default|GetHeld%20Cats) Cat)
  (CallFunction|DisableCat Cat))