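; Player controller for a cat-boxing game, handling camera switching, mouse interaction and the pause menu.
; Space toggles between grabbing and boxing cameras found at BeginPlay; in boxing mode, Enter replaces the box and refills empty cat zones.
; Left-click traces under the cursor to grab BPI_DragAndDrop actors, freeing a grabbed cat's zone, or to open and close boxes in boxing mode.
; Tick drags the held object along the mouse ray.
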(event EventBeginPlay
  (bind _outactors (Actor|GetAllActorsOfClass "/Game/BasicAssets/Cat/BP_CatZone.BP_CatZone_C"))
  (Variables|Default|SetAllCatZones _outactors)
  (bind _outactors_2 (Actor|GetAllActorsOfClass "/Game/BasicAssets/BP_BoxingCamera.BP_BoxingCamera_C"))
  (Variables|Default|SetBoxing%20Camera (Utilities|Array|Get(acopy) _outactors_2))
  (bind _outactors_3 (Actor|GetAllActorsOfClass "/Game/BasicAssets/BP_GrabbingCamera.BP_GrabbingCamera_C"))
  (Variables|Default|SetGrabbing%20Camera (Utilities|Array|Get(acopy) _outactors_3))
  (bind _outactors_4 (Actor|GetAllActorsOfClass "/Game/BasicAssets/BP_BoxingZone.BP_BoxingZone_C"))
  (Variables|Default|SetBoxing%20Zone (Utilities|Array|Get(acopy) _outactors_4))
  (Game|Player|SetViewTargetwithBlend (Variables|Default|GetGrabbing%20Camera) 0.0 "VTBlend_Linear" 0.0 false))

(event EventTick
  (params (DeltaSeconds :type Float%20%28single-precision%29))
  (bind (_worldlocation _worlddirection) (Game|Player|ConvertMouseLocationToWorldSpace))
  (bind _grabbed_thing (Variables|Default|GetGrabbed%20Thing))
  (Utilities|IsValid (Utilities|ToObject(Interface) _grabbed_thing)
    (:Is%20Valid
      (Default|Drag _grabbed_thing (+ _worldlocation (* _worlddirection (Variables|Default|GetDistance%20to%20Dragable)))))))

(event Input|MouseEvents|LeftMouseButton
  (params (Key :type Key%20Structure :default "None"))
  (bind (_worldlocation _worlddirection) (Game|Player|ConvertMouseLocationToWorldSpace))
  (:Pressed
    (bind (_outhit _returnvalue) (Collision|LineTraceByChannel _worldlocation (+ _worldlocation (* _worlddirection 1e+04)) "TraceTypeQuery1" false 0 "Persistent"))
    (if _returnvalue
      (bind _asbpi_drag_and_drop (Utilities|Casting|CastToBPI_DragAndDrop (.HitActor (Collision|BreakHitResult _outhit)))
        (:then
          (bind _output_get (Variables|Default|SetGrabbed%20Thing _asbpi_drag_and_drop))
          (Default|Grabbed _output_get)
          (bind _asbp_cat (Utilities|Casting|CastToBP_Cat _output_get))
          (for _array_element (Variables|Default|GetAllCatZones)
            (bind _isthismycat_ (Default|IsThisMyCat? _array_element _asbp_cat))
            (if _isthismycat_
              (Default|SetCatinZone _array_element false))))
        (:CastFailed
          (if (Variables|Default|GetIAmBoxing?)
            (bind _asbp_box (Utilities|Casting|CastToBP_Box (.HitActor (Collision|BreakHitResult _outhit))))
            (if (Rendering|IsVisible (Variables|/Game/Davis/Blueprints/BP_Box.BP_Box_C|GetBox_Open _asbp_box))
              (Default|BoxClose _asbp_box)
              (else
                (Default|BoxOpen _asbp_box))))))))
  (:Released
    (Utilities|IsValid (Utilities|ToObject(Interface) (Variables|Default|GetGrabbed%20Thing))
      (:Is%20Valid
        (Default|Released (Variables|Default|GetGrabbed%20Thing))))))

(event Input|KeyboardEvents|Escape
  (params (Key :type Key%20Structure :default "None"))
  (:Pressed
    (Utilities|IsValid (Variables|Default|GetPauseMenu)
      (:Is%20Valid
        (Widget|SetVisibility (Variables|Default|GetPauseMenu) "Visible"))
      (:Is%20Not%20Valid
        (bind _returnvalue (UserInterface|CreateWidget "/Game/BasicAssets/JasonMessingArouns/BPW_PawsMenu.BPW_PawsMenu_C" self))
        (bind _output_get (Variables|Default|SetPauseMenu _returnvalue))
        (UserInterface|Viewport|AddtoViewport _output_get 0)))))

(event Input|KeyboardEvents|SpaceBar
  (params (Key :type Key%20Structure :default "None"))
  ;[1 1 1] Handles Camera Swaping
  (:Pressed
    (bind _isa (Utilities|FlowControl|FlipFlop)
      (:A
        (Game|Player|SetViewTargetwithBlend (Variables|Default|GetBoxing%20Camera) 0.5 "VTBlend_Linear" 0.0 false))
      (:B
        (Game|Player|SetViewTargetwithBlend (Variables|Default|GetGrabbing%20Camera) 0.5 "VTBlend_Linear" 0.0 false)))
    (Variables|Default|SetIAmBoxing? _isa)))

(event Input|KeyboardEvents|Enter
  (params (Key :type Key%20Structure :default "None"))
  (bind _boxing_zone (Variables|Default|GetBoxing%20Zone))
  (:Pressed
    (if (Variables|Default|GetIAmBoxing?)
      (Default|DisposeOfBox _boxing_zone)
      (Default|SpawnBox _boxing_zone)
      (for _array_element (Variables|Default|GetAllCatZones)
        (if (not (Variables|/Game/BasicAssets/Cat/BP_CatZone.BP_CatZone_C|GetIsCatInZone _array_element))
          (bind _returnvalue (Game|SpawnActorfromClass "/Game/BasicAssets/Cat/BP_Cat.BP_Cat_C" (Transformation|GetActorTransform _array_element) "Undefined" "MultiplyWithRoot" 0 0))
          (Default|AddCattoZone _array_element _returnvalue))))))

(fn ConstructionScript)

(fn CatReadyforBoxing)

(fn Drag
  (params (Location :type Vector :default "0, 0, 0")))