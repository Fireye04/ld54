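; BP_Cat is a cat actor that receives idle behaviours and currently only prints them, with no movement or animation logic.
; PerformIdle switches on the idle animation to print laying down, stretching, or walking and jumping from the start position to the last path point.
; The construction script randomises and prints cat volume and head size.
; Walk is an empty stub, and its only call is never run.
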(event Custom|PerformIdle
  (params (Is%20Static? :type Boolean) (Idle :type ST%20Cat%20Zone%20Idle%20Structure))
  (bind (_startposition _path _animation) (Utilities|Struct|BreakST_CatZoneIdle Idle))
  (bind _returnvalue (Utilities|Array|Length _path))
  (bind _returnvalue_2 (Utilities|String|ToString(Transform) _startposition))
  (bind _returnvalue_3 (- _returnvalue 1))
  (bind _output (Utilities|Array|Get(acopy) _path _returnvalue_3))
  (bind _returnvalue_4 (Utilities|String|ToString(Transform) _output))
  (switch Utilities|FlowControl|Switch|SwitchonE_CatIdles _animation
    (:NewEnumerator0
      (Development|PrintString "Laying down"))
    (:NewEnumerator1
      (Development|PrintString (Utilities|String|Append "Moving from " _returnvalue_2 " to " _returnvalue_4)))
    (:NewEnumerator2
      (Development|PrintString (Utilities|String|Append "Jumping from " _returnvalue_2 " to " _returnvalue_4)))
    (:NewEnumerator3
      (Development|PrintString "Stretching"))))

(event EventBeginPlay)

(event Collision|EventActorBeginOverlap
  (params (OtherActor :type Actor%20Object%20Reference)))

(fn ConstructionScript
  (bind _output_get (Variables|Default|SetCat%20Volume (Math|Random|RandomIntegerinRange 1 5)))
  (bind _output_get_2 (Variables|Default|SetCatHeadSize (Math|Random|RandomIntegerinRange 1 5)))
  (Development|PrintString (Utilities|String|Append "Cat volume : " (Utilities|String|ToString(Integer) _output_get) " |  Cat head size: " (Utilities|String|ToString(Integer) _output_get_2))))

(fn Walk
  (params (Goal :type Transform)))