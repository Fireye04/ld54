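; BP_PathNode is a cat path waypoint actor that holds a wait duration, a delay animation and a next animation.
; Construction and Regen Vars both roll a random 1–5 integer duration and set the two animation enums to fixed values.
; Get Vars returns those values with the node's transform.
; Regen Vars returns the refreshed values, though its NextAnim output carries DelayAnim and IdleAnims carries NextAnim.
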(event EventBeginPlay)

(event Collision|EventActorBeginOverlap
  (params (OtherActor :type Actor%20Object%20Reference)))

(event EventTick
  (params (DeltaSeconds :type Float%20%28single-precision%29)))

(fn ConstructionScript
  (Variables|Default|SetDelay%20Duration (Math|Random|RandomIntegerinRange 1 5))
  (Variables|Default|SetDelay%20Anim "NewEnumerator1")
  (Variables|Default|SetNext%20Anim "NewEnumerator0"))

(fn GetVars
  (return (Transformation|GetActorTransform self) (Variables|Default|GetDelay%20Anim) (Variables|Default|GetDelay%20Duration) (Variables|Default|GetNext%20Anim)))

(fn RegenVars
  (bind _output_get (Variables|Default|SetDelay%20Duration (Math|Random|RandomIntegerinRange 1 5)))
  (bind _output_get_2 (Variables|Default|SetDelay%20Anim "NewEnumerator1"))
  (bind _output_get_3 (Variables|Default|SetNext%20Anim "NewEnumerator0"))
  (return _output_get _output_get_2 _output_get_3))