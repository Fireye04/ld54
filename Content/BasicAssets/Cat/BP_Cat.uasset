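; BP_Cat is a cat actor that idles along a zone's path nodes under behavior tree control.
; PerformIdle adds the zone's path and start nodes to its node list and runs the tree through ACMoveBehavior; index helpers cycle that list.
; The construction script randomizes volume and head size, summed as the cat's unit count.
; SetCatVisibility only stores a visibility flag.
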(event Custom|PerformIdle
  (params (zone :type ST%20Cat%20Zone%20Structure))
  (bind (_startnode _pathnodes) (Utilities|Struct|BreakST_CatZone zone))
  (bind _output_get (Variables|Default|SetNodeList _pathnodes))
  (Utilities|Array|Add _output_get _startnode)
  (Default|RunBT (Variables|Default|GetAC_MoveBehavior)))

(event EventBeginPlay)

(event Collision|EventActorBeginOverlap
  (params (OtherActor :type Actor%20Object%20Reference)))

(event EventTick
  (params (DeltaSeconds :type Float%20%28single-precision%29)))

(fn ConstructionScript
  (bind _output_get (Variables|Default|SetCat%20Volume (Math|Random|RandomIntegerinRange 1 4)))
  (bind _output_get_2 (Variables|Default|SetCatHeadSize (Math|Random|RandomIntegerinRange 1 4)))
  (Variables|Default|Setindex 0)
  (Development|PrintString (Utilities|String|Append "Cat volume : " (Utilities|String|ToString(Integer) _output_get) " |  Cat head size: " (Utilities|String|ToString(Integer) _output_get_2))))

(fn GetCatUnits
  (return (+ (Variables|Default|GetCatHeadSize) (Variables|Default|GetCat%20Volume))))

(fn SetCatVisibility
  (params (Visibility :type Boolean))
  (Variables|Default|SetIsVisible Visibility))

(fn GetCurrentNode
  (return (Utilities|Array|Get(acopy) (Variables|Default|GetNodeList) (Variables|Default|Getindex))))

(fn IncrementIndex
  (if (< (+ (Variables|Default|Getindex) 1) (Utilities|Array|Length (Variables|Default|GetNodeList)))
    (Variables|Default|Setindex (+ (Variables|Default|Getindex) 1))
    (else
      (Variables|Default|Setindex 0))))