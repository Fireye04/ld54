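; BP_CatZone is an actor defining an idle zone where a resident cat performs an idle routine along path nodes.
; AddCatToZone gathers child BP_PathNode actors, converts their position and delay/animation settings into path structs, then calls PerformIdle on the cat with a zone struct starting at its own transform.
; Adding or removing the cat updates the IsCatInZone flag and passes it to the cat.
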(event Custom|Add%20Cat%20To%20Zone
  (params (Cat :type BP%20Cat%20Object%20Reference))
  (Variables|Default|SetResidentCat Cat)
  (for _array_element (Actor|GetAllChildActors self true)
    (bind _asbp_path_node (Utilities|Casting|CastToBP_PathNode _array_element))
    (Utilities|Array|Add (Variables|Default|GetPath%20nodes) _asbp_path_node))
  (for _array_element_2 (Variables|Default|GetPath%20nodes)
    (bind (_pos _delay_anim _delay_duration _next_anim) (Default|GetVars _array_element_2))
    (Utilities|Array|Add (Variables|Default|GetCat%20Idle%20Path) (Utilities|Struct|MakeST_Node _pos _delay_anim _delay_duration _next_anim)))
  (Default|PerformIdle (Variables|Default|GetResidentCat) (Utilities|Struct|MakeST_CatZone (Utilities|Struct|MakeST_Node (Transformation|GetActorTransform self) (Variables|Default|GetStartDelayAnim) (Variables|Default|GetStartDelayDuration) (Variables|Default|GetStartNextAnim)) (Variables|Default|GetCat%20Idle%20Path)) (Variables|Default|GetPath%20nodes))
  (CallFunction|SetCatinZone true))

(event Custom|Remove%20Cat%20From%20Zone
  ;[1 1 1] TODO
  (CallFunction|SetCatinZone false))

(event EventBeginPlay)

(event Collision|EventActorBeginOverlap
  (params (OtherActor :type Actor%20Object%20Reference)))

(event EventTick
  (params (DeltaSeconds :type Float%20%28single-precision%29)))

(fn ConstructionScript)

(fn SetCatinZone
  (params (in%20Zone :type Boolean))
  (bind _output_get (Variables|Default|SetIsCatInZone in%20Zone))
  (Default|SetZone (Variables|Default|GetResidentCat) _output_get))