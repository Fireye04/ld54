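; BP_BoxingZone is an actor that receives dragged cats for packing into boxes.
; On BeginPlay it gathers the holding spot actors and spawns an open BP_Box at its own transform.
; CatCatcherZone overlaps notify draggables through BPI_DragAndDrop when they enter or leave.
; AddCatForBoxing moves each cat to the spot matching its array index and enables physics, while DisposeOfBox closes the box and pushes it away with a force.
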(event OnComponentBeginOverlap(CatCatcherZone)
  (params (OverlappedComponent :type Primitive%20Component%20Object%20Reference) (OtherActor :type Actor%20Object%20Reference) (OtherComp :type Primitive%20Component%20Object%20Reference) (OtherBodyIndex :type Integer) (bFromSweep :type Boolean) (SweepResult :type Hit%20Result%20Structure%20%28by%20ref%29))
  (bind _asbpi_drag_and_drop (Utilities|Casting|CastToBPI_DragAndDrop OtherActor))
  (Default|OverBoxingArea _asbpi_drag_and_drop))

(event OnComponentEndOverlap(CatCatcherZone)
  (params (OverlappedComponent :type Primitive%20Component%20Object%20Reference) (OtherActor :type Actor%20Object%20Reference) (OtherComp :type Primitive%20Component%20Object%20Reference) (OtherBodyIndex :type Integer))
  (bind _asbpi_drag_and_drop (Utilities|Casting|CastToBPI_DragAndDrop OtherActor))
  (Default|OutOfBoxingArea _asbpi_drag_and_drop))

(event EventBeginPlay
  (bind _outactors (Actor|GetAllActorsOfClass "/Game/BasicAssets/BP_CatForBoxingHoldingSpot.BP_CatForBoxingHoldingSpot_C"))
  (Variables|Default|SetCatsForBoxingSpots _outactors)
  (CallFunction|SpawnBox))

(event Collision|EventActorBeginOverlap
  (params (OtherActor :type Actor%20Object%20Reference)))

(event EventTick
  (params (DeltaSeconds :type Float%20%28single-precision%29)))

(fn ConstructionScript)

(fn AddCatforBoxing
  (params (CatToBox :type BP%20Cat%20Object%20Reference) (Physics%20Component :type Mesh%20Component%20Object%20Reference))
  (bind _returnvalue (Utilities|Array|Add (Variables|Default|GetCatsForBoxing) CatToBox))
  (Transformation|SetActorTransform CatToBox (Transformation|GetActorTransform (Utilities|Array|Get(acopy) (Variables|Default|GetCatsForBoxingSpots) _returnvalue)))
  (Physics|SetSimulatePhysics Physics%20Component true))

(fn SpawnBox
  (bind _returnvalue (Game|SpawnActorfromClass "/Game/Davis/Blueprints/BP_Box.BP_Box_C" (Transformation|GetActorTransform) "Undefined" "MultiplyWithRoot" 0 0))
  (bind _output_get (Variables|Default|SetCurrentBox _returnvalue))
  (Default|BoxOpen _output_get))

(fn DisposeOfBox
  (bind _currentbox (Variables|Default|GetCurrentBox))
  (bind _box_closed (Variables|/Game/Davis/Blueprints/BP_Box.BP_Box_C|GetBox_Closed _currentbox))
  (Default|BoxClose _currentbox)
  (Physics|SetSimulatePhysics _box_closed true)
  (Physics|AddForce _box_closed "150.000000,0.000000,100.000000" "None" false))