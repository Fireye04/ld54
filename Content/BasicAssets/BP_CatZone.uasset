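; BP_CatZone is a zone actor that tracks a single resident cat.
; AddCatToZone stores the given cat as ResidentCat and prints its display name, and RemoveCatFromZone clears the reference.
; An unconnected, never-run chain would wait briefly, then make the cat perform an idle built from the zone and cat transforms.
; BeginPlay, overlap and Tick do nothing.
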(event Custom|Add%20Cat%20To%20Zone
  (params (Cat :type BP%20Cat%20Object%20Reference))
  (bind _output_get (Variables|Default|SetResidentCat Cat))
  (Development|PrintString (Utilities|GetDisplayName _output_get)))

(event Custom|Remove%20Cat%20From%20Zone
  (Variables|Default|SetResidentCat 0))

(event EventBeginPlay)

(event Collision|EventActorBeginOverlap
  (params (OtherActor :type Actor%20Object%20Reference)))

(event EventTick
  (params (DeltaSeconds :type Float%20%28single-precision%29)))

(fn ConstructionScript)