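; BP_Box is a box actor that can show either an open or a closed state.
; It holds two components, BoxOpen and BoxClosed, both set visible on BeginPlay, with the open one hidden so the box starts closed.
; The BoxOpen and BoxClose events swap states by toggling Hidden In Game on the two components.
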(event Custom|BoxClose
  (Development|SetHiddeninGame (Variables|Default|GetBox_Closed) false false)
  (Development|SetHiddeninGame (Variables|Default|GetBox_Open) true false))

(event Custom|BoxOpen
  (Development|SetHiddeninGame (Variables|Default|GetBox_Closed) true false)
  (Development|SetHiddeninGame (Variables|Default|GetBox_Open) false false))

(event EventBeginPlay
  (Rendering|SetVisibility (Variables|Default|GetBox_Open) true false)
  (Development|SetHiddeninGame (Variables|Default|GetBox_Open) true false))

(fn ConstructionScript)